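; AI controller for the Sedan_AI_BP vehicle that sets throttle and steering to avoid obstacles.
; Each tick line-traces ahead from above the car, with debug drawing.
; A hit triggers a DoOnce-gated reverse with turn, rechecked every second until clear, then drives straight forward.
; Drive and Steer events pass these values to the vehicle, but their looping timers are unconnected, so nothing here calls them.
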(event `Drive`
  ;[1 1 1] Drive
  (`/Game/Blueprints/Sedan/Sedan_AI_BP.Throttle` (`self.ControlledVehicle`) (`self.Throttle`)))

(event `Steer`
  ;[1 1 1] Steer
  (`/Game/Blueprints/Sedan/Sedan_AI_BP.Steering` (`self.ControlledVehicle`) (`self.Steering`)))

(event `self.ReceiveBeginPlay`
  ;[1 1 1] BeginPlay
  ;;[0.1244 0 1] BeginPlay
  (bind _assedan_ai_bp (cast `/Game/Blueprints/Sedan/Sedan_AI_BP` (`self.K2_GetPawn`)))
  (set `self.ControlledVehicle` _assedan_ai_bp))

(event `Reverse`
  (`/Engine/EditorBlueprintResources/StandardMacros.DoOnce` false :!label _label
    (:`Completed`
      (set `self.Throttle` -1.0)
      (set `self.Steering` -1.0)
      (`KismetSystemLibrary.Delay` 1.0 :!label _label_2)
      (if (`self.Hitting?`)
        (goto _label_2)
        (else
          (set `self.Throttle` 1.0)
          (set `self.Steering` 0.0))))))

(event `self.ReceiveTick`
  (params (DeltaSeconds :type "Float (single-precision)"))
  (bind _hit (`self.-Trace` 1000.0))
  (bind _output_get (set `self.Hitting?` _hit))
  (if _output_get
    (`self.Reverse`)
    (else
      (goto _label :!via `Reset`))))

(fn `-Trace`
  (params (Distance :type "Float (double-precision)"))
  (returns (Hit :type Boolean))
  (bind _controlledvehicle (`self.ControlledVehicle`))
  (bind _returnvalue (`KismetMathLibrary.MakeVector` (.x (`self.K2_GetActorLocation` _controlledvehicle)) (.y (`self.K2_GetActorLocation` _controlledvehicle)) (+ (.z (`self.K2_GetActorLocation` _controlledvehicle)) 150.0)))
  (bind (_outhit _returnvalue_2) (`KismetSystemLibrary.LineTraceSingleForObjects` _returnvalue (+ _returnvalue (* (`self.GetActorForwardVector` _controlledvehicle) Distance)) (`|MakeArray` "ObjectTypeQuery1" "ObjectTypeQuery2" :!type "EObjectTypeQuery Enum") false (`|MakeArray` (`self.ControlledVehicle`) :!type "Actor Object Reference") "ForOneFrame"))
  (return _returnvalue_2))

(fn `UserConstructionScript`)